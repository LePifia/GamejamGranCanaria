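; BP_FantasmaBueno is a friendly ghost actor that starts a dialogue when the third-person character overlaps its box.
; The overlap disables player input, then removes any existing dialogue widget or creates a WB_Dialogo.
; A new widget receives the ghost's Dialogue text and Doors reference and is added to the viewport.
; The ghost destroys itself after showing the widget, leaving input disabled on its side.
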(event OnComponentBeginOverlap(Box)
  (params (OverlappedComponent :type Primitive%20Component%20Object%20Reference) (OtherActor :type Actor%20Object%20Reference) (OtherComp :type Primitive%20Component%20Object%20Reference) (OtherBodyIndex :type Integer) (bFromSweep :type Boolean) (SweepResult :type Hit%20Result%20Structure%20%28by%20ref%29))
  (bind _returnvalue (Game|GetPlayerController 0))
  (Utilities|Casting|CastToBP_ThirdPersonCharacter OtherActor)
  (Input|DisableInput (Pawn|GetControlledPawn _returnvalue) _returnvalue)
  (if (Utilities|IsValid (Variables|Default|GetCurrentWidget))
    (Widget|RemovefromParent (Variables|Default|GetCurrentWidget))
    (Variables|Default|SetCurrentWidget 0)
    (else
      (bind _returnvalue_2 (UserInterface|CreateWidget "/Game/Blueprint/Elsa/WB_Dialogo.WB_Dialogo_C" (Game|GetPlayerController 0)))
      (Variables|Default|SetCurrentWidget _returnvalue_2)
      (Variables|/Game/Blueprint/Elsa/WB_Dialogo.WB_Dialogo_C|SetDisplayText (Variables|Default|GetCurrentWidget) (Variables|Default|GetDialogue))
      (Variables|/Game/Blueprint/Elsa/WB_Dialogo.WB_Dialogo_C|SetDoor (Variables|Default|GetCurrentWidget) (Variables|Default|GetDoors))
      (UserInterface|Viewport|AddtoViewport (Variables|Default|GetCurrentWidget) 0)
      (Actor|DestroyActor))))

(fn ConstructionScript)