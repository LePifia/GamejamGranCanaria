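; GI_Persistente, by its name a persistent Game Instance, runs a global countdown that sends the game to Level_1 when time runs out.
; E_IniciarTimer starts a looping one-second timer and stores its handle, and each tick of E_resta decrements TiempoRestante.
; At zero it clears the timer, resets the remaining time to five minutes and opens the level, without restarting the timer itself.
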(event Custom|E_resta
  (Variables|Default|SetTiempoRestante (- (Variables|Default|GetTiempoRestante) 1.0))
  (if (<= (Variables|Default|GetTiempoRestante) 0.0)
    (Utilities|Time|ClearandInvalidateTimerbyHandle (Variables|Default|GetTimerHandle_Global))
    (Variables|Default|SetTiempoRestante 3e+02)
    (Game|OpenLevel(byObjectReference) "/Game/ThirdPerson/Maps/Level_1.Level_1")))

(event Custom|E_IniciarTimer
  (bind _returnvalue (Utilities|Time|SetTimerbyEvent (delegate Custom|E_resta) 1.0 true))
  (Variables|Default|SetTimerHandle_Global _returnvalue))