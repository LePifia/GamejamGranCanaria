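; BP_Door is a door that the third-person character opens by walking into its trigger box, playing a sound and disabling the cube's collision.
; Doors flagged GoodDoor open only when CanOpenDoor is set; otherwise they disable player input and show the WB_NotPas widget.
; Other doors always open.
; A second box, Box1, loads LevelName as a level instance when the character enters it, but only on good doors.
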(event OnComponentBeginOverlap(Box)
  (params (OverlappedComponent :type Primitive%20Component%20Object%20Reference) (OtherActor :type Actor%20Object%20Reference) (OtherComp :type Primitive%20Component%20Object%20Reference) (OtherBodyIndex :type Integer) (bFromSweep :type Boolean) (SweepResult :type Hit%20Result%20Structure%20%28by%20ref%29))
  (bind _returnvalue (Game|GetPlayerController 0))
  (Utilities|Casting|CastToBP_ThirdPersonCharacter OtherActor)
  (if (Variables|Default|GetGoodDoor)
    (if (Variables|Default|GetCanOpenDoor)
      (Audio|PlaySound2D 0 1.0 1.0 0.0 0 0 :!label _label)
      (Collision|SetCollisionEnabled (Variables|Default|GetCube) "NoCollision")
      (else
        (Input|DisableInput (Pawn|GetControlledPawn _returnvalue) _returnvalue)
        (bind _returnvalue_2 (UserInterface|CreateWidget "/Game/Blueprint/Elsa/WB_NotPas.WB_NotPas_C" (Game|GetPlayerController 0)))
        (Variables|Default|SetCurrentWidget _returnvalue_2)
        (UserInterface|Viewport|AddtoViewport (Variables|Default|GetCurrentWidget) 0)))
    (else
      (goto _label))))

(event OnComponentBeginOverlap(Box1)
  (params (OverlappedComponent :type Primitive%20Component%20Object%20Reference) (OtherActor :type Actor%20Object%20Reference) (OtherComp :type Primitive%20Component%20Object%20Reference) (OtherBodyIndex :type Integer) (bFromSweep :type Boolean) (SweepResult :type Hit%20Result%20Structure%20%28by%20ref%29))
  (Utilities|Casting|CastToBP_ThirdPersonCharacter OtherActor)
  (if (Variables|Default|GetGoodDoor)
    (Class|LevelStreamingDynamic|LoadLevelInstance (Variables|Default|GetLevelName) "0, 0, 0" "0, 0, 0" "" 0 false)))

(fn ConstructionScript)