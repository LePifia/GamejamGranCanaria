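; Enemy phantom that patrols between linked target points, chases the player on perception and damages them on contact.
; An AI MoveTo loop follows each BPNextTarget's next-target reference to advance the patrol.
; Any perception update plays a 2D sound, then issues a move toward the actor if it is the ThirdPersonCharacter.
; Overlapping the death collision applies damage to that character, gated by a DoOnce that is never reset.
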(event OnComponentBeginOverlap(DeadCollsion)
  (params (OverlappedComponent :type Primitive%20Component%20Object%20Reference) (OtherActor :type Actor%20Object%20Reference) (OtherComp :type Primitive%20Component%20Object%20Reference) (OtherBodyIndex :type Integer) (bFromSweep :type Boolean) (SweepResult :type Hit%20Result%20Structure%20%28by%20ref%29))
  ;[1 1 1] On collision Reset Level
  (bind _asbp_third_person_character (Utilities|Casting|CastToBP_ThirdPersonCharacter OtherActor))
  (Variables|Default|SetAs%20BP%20Third%20Person%20Character _asbp_third_person_character)
  (Utilities|FlowControl|DoOnce false
    (:Completed
      (Game|Damage|ApplyDamage _asbp_third_person_character 1.0 0 0)
      (Development|PrintString "Hello"))))

(event OnTargetPerceptionUpdated(AIPerception)
  (params (Actor :type Actor%20Object%20Reference) (Stimulus :type AI%20Stimulus%20Structure))
  ;[1 1 1] If Detected By Looking, it would chase the player
  (Development|PrintString "DETECTED")
  (Audio|PlaySound2D 0 1.0 1.0 0.0 0 0)
  (bind _asbp_third_person_character (Utilities|Casting|CastToBP_ThirdPersonCharacter Actor))
  (AI|AIMoveTo (AI|GetAIController self) "0, 0, 0" _asbp_third_person_character -1.0 "Default" "Default" true true))

(event EventBeginPlay
  ;[1 1 1] Patrol Between Different Points
  (AI|AIMoveTo (AI|GetAIController self) (Transformation|GetWorldLocation (Variables|/Game/Blueprint/David/BPNextTarget.BPNextTarget_C|GetSphere (Variables|Default|GetTargetPoint))) 0 -1.0 "Default" "Default" true true :!label _label
    (:OnMoveFinished
      (bind _asbpnext_target (Utilities|Casting|CastToBPNextTarget (Variables|Default|GetTargetPoint)))
      (Variables|Default|SetTargetPoint (Variables|/Game/Blueprint/David/BPNextTarget.BPNextTarget_C|GetBpNextTarget _asbpnext_target))
      (goto _label))))

(fn ConstructionScript)