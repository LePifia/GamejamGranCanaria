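; BP_EnemyPhantomTP is an enemy phantom that chases the third-person player and damages them on contact.
; AI perception updates play a sound and start an AIMoveTo chase while HasDetectedPlayer is false; this file never sets that flag.
; Tick faces the player if the flag is set and moves back to DefaultPos when the player is over 1000 units away.
; A looping target-point patrol exists but is unconnected.
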(event OnComponentBeginOverlap(DeadCollsion)
  (params (OverlappedComponent :type Primitive%20Component%20Object%20Reference) (OtherActor :type Actor%20Object%20Reference) (OtherComp :type Primitive%20Component%20Object%20Reference) (OtherBodyIndex :type Integer) (bFromSweep :type Boolean) (SweepResult :type Hit%20Result%20Structure%20%28by%20ref%29))
  ;[1 1 1] On collision Reset Level
  (bind _asbp_third_person_character (Utilities|Casting|CastToBP_ThirdPersonCharacter OtherActor))
  (Utilities|FlowControl|Delay 0.5)
  (Game|Damage|ApplyDamage _asbp_third_person_character 1.0 0 0))

(event OnTargetPerceptionUpdated(AIPerception)
  (params (Actor :type Actor%20Object%20Reference) (Stimulus :type AI%20Stimulus%20Structure))
  ;[1 1 1] If Detected By Looking, it would chase the player
  (Development|PrintString "DETECTED")
  (Audio|PlaySound2D 0 1.0 1.0 0.0 0 0)
  (if (not (Variables|Default|GethasDetectedPlayer))
    (bind _asbp_third_person_character (Utilities|Casting|CastToBP_ThirdPersonCharacter Actor))
    (bind _output_get (Variables|Default|SetAs%20BP%20Third%20Person%20Character _asbp_third_person_character))
    (bind _output_get_2 (Variables|Default|Settarget%20actor _output_get))
    (AI|AIMoveTo (AI|GetAIController self) (Transformation|GetActorLocation (Variables|Default|GetAs%20BP%20Third%20Person%20Character)) _output_get_2 -1.0 "Default" "Default" true true)))

(event EventBeginPlay
  ;[1 1 1] Patrol Between Different Points
)

(event EventTick
  (params (DeltaSeconds :type Float%20%28single-precision%29))
  (bind _as_bp_third_person_character (Variables|Default|GetAs%20BP%20Third%20Person%20Character))
  (Utilities|FlowControl|Sequence
    (:then_0
      (if (Variables|Default|GethasDetectedPlayer)
        (Transformation|SetActorRotation (Math|Rotator|FindLookatRotation (Transformation|GetActorLocation self) (Transformation|GetActorLocation (Variables|Default|GetAs%20BP%20Third%20Person%20Character))))))
    (:then_1
      (Utilities|IsValid _as_bp_third_person_character
        (:Is%20Valid
          (if (not (<= (Math|Vector|Distance(Vector) (Transformation|GetWorldLocation (Variables|Character|GetMesh self)) (Transformation|GetWorldLocation (Variables|/Script/Engine.Character|GetMesh _as_bp_third_person_character))) 1e+03))
            (AI|AIMoveTo (AI|GetAIController self) "0, 0, 0" (Variables|Default|GetdefaultPos) -1.0 "Default" "Default" true true)))))))

(fn ConstructionScript)